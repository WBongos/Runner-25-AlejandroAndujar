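; Bullet actor that travels in a straight line and can kill the player.
; Each Tick it sets the actor location to the Cube's world position offset along world X by MSpeed scaled by delta time, without sweep.
; A Death function checks whether the passed actor is the first player's character, then destroys it and prints a death message; nothing in this file calls it.
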(event EventTick
  (params (DeltaSeconds :type Float%20%28single-precision%29))
  (Transformation|SetActorLocation (+ (Transformation|GetWorldLocation (Variables|Default|GetCube)) (Math|Vector|MakeVector (* DeltaSeconds (Variables|Default|GetmSpeed)) 0.0 0.0)) false false))

(fn ConstructionScript)

(fn Death
  (params (Player :type Actor%20Object%20Reference))
  (bind _returnvalue (Game|GetPlayerCharacter 0))
  (if (== Player _returnvalue)
    (Actor|DestroyActor _returnvalue)
    (Development|PrintText "Muerto")))