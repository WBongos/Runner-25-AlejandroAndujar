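; BP_Point is a moving score trigger that awards a point when the player character overlaps its cube.
; The overlap increments the BP_GS game state's point count and fires its OnPoint dispatcher.
; Tick moves it along negative X at a speed copied from BP_GS when put in use or on a difficulty raise.
; The game state's death event takes it out of use through the inherited Use event and zeroes its speed.
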(event OnComponentBeginOverlap(Cube1)
  (params (OverlappedComponent :type Primitive%20Component%20Object%20Reference) (OtherActor :type Actor%20Object%20Reference) (OtherComp :type Primitive%20Component%20Object%20Reference) (OtherBodyIndex :type Integer) (bFromSweep :type Boolean) (SweepResult :type Hit%20Result%20Structure%20%28by%20ref%29))
  ;[1 0.6347 0.4036] CallOnPoint
  (if (== OtherActor (Game|GetPlayerCharacter 0))
    (bind _asbp_gs (Utilities|Casting|CastToBP_GS (Game|GetGameState)))
    (bind _result (Math|Float|IncrementFloat (Variables|/Game/Blueprints/BP_GS.BP_GS_C|GetmPoints _asbp_gs))
      (:%20%20
        (Default|CallOnPoint _asbp_gs _result)))))

(event Custom|OnDeathEvent
  ;[0 0.4534 1] BindOnDeath
  (CallFunction|Use false)
  (Variables|Default|SetmSpeed 0.0))

(event Custom|IncreaseSpeed
  ;[0.1597 1 0] BindOnDifficultyIncrease
  (Variables|Default|SetmSpeed (Variables|/Game/Blueprints/BP_GS.BP_GS_C|GetmSpeed (stale EventBeginPlay _asbp_gs_2))))

(event EventTick
  (params (DeltaSeconds :type Float%20%28single-precision%29))
  ;[0.275 1 0.7961] Movement
  (Transformation|SetActorLocation (+ (* (* (Variables|Default|GetmSpeed) "-1.000000,0.000000,0.000000") DeltaSeconds) (Transformation|GetActorLocation)) false false))

(event EventUse
  (params (Use :type Boolean))
  ;[0 0.6573 1] InitialMSpeed
  (|CallParentFunction Use)
  (if Use
    (bind _asbp_gs (Utilities|Casting|CastToBP_GS (Game|GetGameState)))
    (Variables|Default|SetmSpeed (Variables|/Game/Blueprints/BP_GS.BP_GS_C|GetmSpeed _asbp_gs))))

(event EventBeginPlay
  (Utilities|FlowControl|Sequence
    (:then_0
      ;[0 0.4534 1] BindOnDeath
      (bind _asbp_gs (Utilities|Casting|CastToBP_GS (Game|GetGameState)))
      (EventDispatchers|BindEventtoOnDeath _asbp_gs (delegate Custom|OnDeathEvent)))
    (:then_1
      ;[0.1597 1 0] BindOnDifficultyIncrease
      (bind _asbp_gs_2 (Utilities|Casting|CastToBP_GS (Game|GetGameState)))
      (EventDispatchers|BindEventtoOnDifficultyRaise _asbp_gs_2 (delegate Custom|IncreaseSpeed)))))

(fn ConstructionScript)