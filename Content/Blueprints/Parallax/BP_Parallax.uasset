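; BP_Parallax is a looping parallax layer actor that scrolls continuously along negative X.
; Each Tick, the Move function offsets its location by MSpeed scaled by delta time, without sweeping.
; Once it passes a hard-coded left X limit, it jumps back to a fixed position on the right to repeat the scroll.
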(event EventTick
  (params (DeltaSeconds :type Float%20%28single-precision%29))
  (Utilities|FlowControl|Sequence
    (:then_0
      (CallFunction|Move DeltaSeconds))
    (:then_1
      (if (<= (.x (Transformation|GetActorLocation)) -1637.0)
        (Transformation|SetActorLocation (Math|Vector|MakeVector (+ 1.92e+03 2202.1) -6e+01 0.0) false false)))))

(fn ConstructionScript)

(fn Move
  (params (Tick :type Float%20%28double-precision%29))
  (Transformation|SetActorLocation (+ (* (* (Variables|Default|GetmSpeed) "-1.000000,0.000000,0.000000") Tick) (Transformation|GetActorLocation)) false false))