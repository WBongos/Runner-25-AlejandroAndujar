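; BP_GS, apparently the game state, holds points and speed and ramps up difficulty as the score climbs.
; On BeginPlay it binds Reset to OnDeath, restoring starting values, and IncreaseDifficulty to OnPoint.
; When points exactly equal the current threshold and speed is not at its cap, it raises both threshold and speed by fixed steps, then broadcasts OnDifficultyRaise.
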(event Custom|Reset
  ;[0.9582 0.1605 1] Reset
  (Variables|Default|SetmPoints 0.0)
  (Variables|Default|SetmSpeed 5e+02)
  (Variables|Default|SetmaxPoints 1e+01))

(event Custom|IncreaseDifficulty
  (params (Point :type Float%20%28double-precision%29))
  ;[0.5377 0.2389 1] IncreaseDifficulty
  (if (== (Variables|Default|GetmPoints) (Variables|Default|GetmaxPoints))
    (if (not (== (Variables|Default|GetmSpeed) (Variables|Default|GetmaxSpeed)))
      (Variables|Default|SetmaxPoints (+ (Variables|Default|GetmaxPoints) 1e+01))
      (Variables|Default|SetmSpeed (+ (Variables|Default|GetmSpeed) 5e+01))
      (Default|CallOnDifficultyRaise))))

(event EventBeginPlay
  (Utilities|FlowControl|Sequence
    (:then_0
      ;[0.9582 0.1605 1] Reset
      (EventDispatchers|BindEventtoOnDeath (delegate Custom|Reset)))
    (:then_1
      ;[0.5377 0.2389 1] IncreaseDifficulty
      (EventDispatchers|BindEventtoOnPoint (delegate Custom|IncreaseDifficulty)))))

(fn ConstructionScript)